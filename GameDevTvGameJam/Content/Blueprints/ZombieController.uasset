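; Zombie character AI that wanders at random and chases the player character on sight.
; It stands still for a short wake-up delay, then flags the wake-up animation as finished in ABP_Zombie and enables walking.
; Tick uses a random Delay to pace moves to nearby reachable points while no enemy is visible.
; PawnSensing starts the chase and sets CanSeeEnemy, which a short retriggerable delay clears once sightings stop.
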(event OnSeePawn(PawnSensing)
  (params (Pawn :type Pawn%20Object%20Reference))
  (bind _asbp_third_person_character (Utilities|Casting|CastToBP_ThirdPersonCharacter Pawn))
  (Utilities|FlowControl|Sequence
    (:then_0
      (Variables|Default|SetCanSeeEnemy true)
      (AI|AIMoveTo self "0, 0, 0" _asbp_third_person_character 5.0 false))
    (:then_1
      (Utilities|FlowControl|RetriggerableDelay 0.2)
      (Variables|Default|SetCanSeeEnemy false))))

(event EventBeginPlay
  (bind _charactermovement (Variables|Character|GetCharacterMovement))
  (Variables|/Script/Engine.CharacterMovementComponent|SetMaxWalkSpeed _charactermovement 0.0)
  (Utilities|FlowControl|Delay 3.0)
  (bind _asabp_zombie (Utilities|Casting|CastToABP_Zombie (Components|SkeletalMesh|GetAnimInstance (Variables|Character|GetMesh))))
  (Variables|/Game/Animations/ABP_Zombie.ABP_Zombie_C|SetWokeUpAnimationFinished _asabp_zombie true)
  (Variables|/Script/Engine.CharacterMovementComponent|SetMaxWalkSpeed _charactermovement 3e+02))

(event Collision|EventActorBeginOverlap
  (params (OtherActor :type Actor%20Object%20Reference)))

(event EventTick
  (params (DeltaSeconds :type Float%20%28single-precision%29))
  (if (not (Variables|Default|GetCanSeeEnemy))
    (Utilities|FlowControl|Delay (Math|Random|RandomFloatinRange 2.0 5.0))
    (AI|AIMoveTo (AI|GetAIController 0) (.RandomLocation (AI|Navigation|GetRandomReachablePointinRadius (Transformation|GetActorLocation) 5e+02 0 0)) 0 -1.0 "Default" "Default" true true)))

(fn ConstructionScript)