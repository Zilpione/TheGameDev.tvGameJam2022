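; Pedestrian actor that reacts to damage with a sound, infection or ragdoll death.
; Each hit lowers health, and reaching zero turns on physics simulation for the Human mesh and prints a debug message.
; The first non-lethal hit marks it infected, then after a random delay scaled by infection time sets the death flag on its ABP_Pedestran animation instance.
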(event EventBeginPlay
  (Variables|Default|SetHealth 1e+02)
  (Variables|Default|SetInfectionTime 5.0))

(event Collision|EventActorBeginOverlap
  (params (OtherActor :type Actor%20Object%20Reference)))

(event EventTick
  (params (DeltaSeconds :type Float%20%28single-precision%29)))

(event Game|Damage|EventAnyDamage
  (params (Damage :type Float%20%28single-precision%29) (DamageType :type Damage%20Type%20Object%20Reference) (InstigatedBy :type Controller%20Object%20Reference) (DamageCauser :type Actor%20Object%20Reference))
  (bind _output_get (Variables|Default|SetHealth (- (Variables|Default|GetHealth) Damage)))
  (Audio|PlaySoundatLocation "/Game/StarterContent/Audio/Collapse01.Collapse01" (Transformation|GetActorLocation) "0, 0, 0" 1.0 1.0 0.0 0 0 0 0)
  (if (<= _output_get 0.0)
    (Development|PrintString "Morto")
    (Physics|SetSimulatePhysics (Variables|Default|GetHuman) true)
    (elif (not (Variables|Default|GetInfected))
      (Variables|Default|SetInfected true)
      (Utilities|FlowControl|Delay (* (Math|Random|RandomFloat) (Variables|Default|GetInfectionTime)))
      (bind _aspedestran_abp (Utilities|Casting|CastToABP_Pedestran (Components|SkeletalMesh|GetAnimInstance (Variables|Default|GetHuman))))
      (Variables|/Game/Animations/ABP_Pedestran.ABP_Pedestran_C|SetIsDeath _aspedestran_abp true))))

(fn ConstructionScript)