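; Pedestrian character that patrols waypoints, flees threats and turns into a zombie when infected.
; Non-lethal damage sets Infected, then a random delay triggers the death animation; once IsUndead is set, Tick swaps mesh and AnimBP.
; Box overlap with infected pedestrians or the player triggers a scream and speed boost, randomly adding a run to a fixed escape point.
; Zombies wander randomly and use PawnSensing to chase and attack uninfected pedestrians.
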(event OnComponentBeginOverlap(Box)
  (params (OverlappedComponent :type Primitive%20Component%20Object%20Reference) (OtherActor :type Actor%20Object%20Reference) (OtherComp :type Primitive%20Component%20Object%20Reference) (OtherBodyIndex :type Integer) (bFromSweep :type Boolean) (SweepResult :type Hit%20Result%20Structure%20%28by%20ref%29))
  (if (not (Variables|Default|GetTurned)) ; IS ZOMBIE
    (bind _asbp_pedestrian (Utilities|Casting|CastToBP_Pedestrian OtherActor)
      (:then
        (if (Variables|BP_Pedestrian_C|GetInfected _asbp_pedestrian) ; Pedone vede uno zombi
          (Utilities|Run4YourLife _asbp_pedestrian (stale _asbp_third_person_character) :!label _label)))
      (:CastFailed
        (bind _asbp_third_person_character (Utilities|Casting|CastToBP_Player OtherActor))
        (goto _label)))))

(event OnSeePawn(PawnSensing)
  (params (Pawn :type Pawn%20Object%20Reference))
  (bind _asbp_pedestrian (Utilities|Casting|CastToBP_Pedestrian Pawn))
  (if (Variables|Default|GetTurned) ; IS ZOMBIE
    (if (not (Variables|BP_Pedestrian_C|GetInfected _asbp_pedestrian)) ; Zombie Vede un Infetto
      (Utilities|ChaseandAttack _asbp_pedestrian))))

(event Custom|CustomEvent
  (params (OverlappedComponent :type Primitive%20Component%20Object%20Reference) (OtherActor :type Actor%20Object%20Reference) (OtherComp :type Primitive%20Component%20Object%20Reference) (OtherBodyIndex :type Integer) (bFromSweep :type Boolean) (SweepResult :type Hit%20Result%20Structure%20%28by%20ref%29)))

(event EventBeginPlay
  (Variables|Default|SetEscapePoint "-2991.711670,-671.604370,2.252405")
  (Variables|Default|SetHealth 1e+02)
  (Variables|Default|SetInfectionTime 5.0)
  (Variables|/Script/Engine.CharacterMovementComponent|SetMaxWalkSpeed (Variables|Character|GetCharacterMovement) 1.5e+02)
  (Variables|Default|SetOrigin (Transformation|GetActorLocation))
  (if (Variables|Default|GetInfected)
    (Utilities|GetRandomDelay)
    (Utilities|TriggerDeadAnimation)
    (else
      (Utilities|Patrol))))

(event Collision|EventActorBeginOverlap
  (params (OtherActor :type Actor%20Object%20Reference)))

(event EventTick
  (params (DeltaSeconds :type Float%20%28single-precision%29))
  (if (Variables|Default|GetTurned) ; IS ZOMBIE
    (Utilities|ZombieEventTick)
    (else
      (Utilities|PedestrianEventTick))))

(event Game|Damage|EventAnyDamage
  (params (Damage :type Float%20%28single-precision%29) (DamageType :type Damage%20Type%20Object%20Reference) (InstigatedBy :type Controller%20Object%20Reference) (DamageCauser :type Actor%20Object%20Reference))
  (if (Variables|Default|GetTurned) ; IS ZOMBIE
    (Development|PrintString "I am a zombie")
    (else
      (bind _isdead (CallFunction|ApplyDmg Damage))
      (if _isdead
        (Development|PrintString "Morto")
        (Physics|SetSimulatePhysics (Variables|Character|GetMesh) false)
        (else
          (Variables|Default|SetInfected true)
          (Utilities|GetRandomDelay)
          (Utilities|TriggerDeadAnimation))))))

(fn ConstructionScript)

(fn ApplyDmg
  (params (Damage :type Float%20%28double-precision%29))
  (bind _output_get (Variables|Default|SetHealth (- (Variables|Default|GetHealth) Damage)))
  (Audio|PlaySoundatLocation "/Game/Audio/Grunt.Grunt" (Transformation|GetActorLocation) "0, 0, 0" 1.0 1.0 0.0 0 0 0 0)
  (return (<= _output_get 0.0)))

(fn Attack
  (Variables|Default|SetCanSeeEnemy false)
  (Animation|PlayAnimMontage "/Game/Animations/AttackMove.AttackMove" 1.0 "None"))

(fn LookAway
  (params (Away%20From :type Actor%20Object%20Reference))
  (bind _returnvalue (Transformation|GetActorLocation Away%20From))
  (bind _returnvalue_2 (Transformation|GetActorLocation))
  (bind _returnvalue_3 (Math|Rotator|FindLookatRotation _returnvalue_2 _returnvalue))
  (bind _returnvalue_4 (Math|Vector|GetForwardVector _returnvalue_3))
  (bind _returnvalue_5 (* _returnvalue_4 2e+02))
  (bind _returnvalue_6 (+ _returnvalue_2 _returnvalue_5))
  (bind (_x _y) (Math|Vector|BreakVector _returnvalue_6))
  (return (Math|Vector|MakeVector _x _y (.Z (Math|Vector|BreakVector _returnvalue_2)))))