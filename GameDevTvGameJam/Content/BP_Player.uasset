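; Player character Blueprint, animated by a zombie AnimBP, that handles the opening wake-up, sprinting and attack input.
; On BeginPlay it plays a 2D sound and zeroes walk speed, then after a delay flags the wake-up animation finished in ABP_Zombie and restores walking.
; Left Shift toggles sprint speed directly, even during the wake-up delay.
; Left mouse plays the attack montage, with no hit logic here.
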(event EventBeginPlay
  (bind _charactermovement (Variables|Character|GetCharacterMovement))
  (Audio|PlaySound2D "/Game/Audio/Game1.Game1" 0.1 1.0 0.0 0 0)
  (Variables|/Script/Engine.CharacterMovementComponent|SetMaxWalkSpeed _charactermovement 0.0)
  (Utilities|FlowControl|Delay 3.0)
  (bind _asabp_zombie (Utilities|Casting|CastToABP_Zombie (Components|SkeletalMesh|GetAnimInstance (Variables|Character|GetMesh))))
  (Variables|/Game/Animations/ABP_Zombie.ABP_Zombie_C|SetWokeUpAnimationFinished _asabp_zombie true)
  (Variables|/Script/Engine.CharacterMovementComponent|SetMaxWalkSpeed _charactermovement 3e+02))

(event Collision|EventActorBeginOverlap
  (params (OtherActor :type Actor%20Object%20Reference)))

(event EventTick
  (params (DeltaSeconds :type Float%20%28single-precision%29)))

(event Input|KeyboardEvents|LeftShift
  (params (Key :type Key%20Structure :default "None"))
  (bind _charactermovement (Variables|Character|GetCharacterMovement))
  ;[1 1 1] Shift Sprint
  (:Pressed
    (Variables|/Script/Engine.CharacterMovementComponent|SetMaxWalkSpeed _charactermovement 6e+02))
  (:Released
    (Variables|/Script/Engine.CharacterMovementComponent|SetMaxWalkSpeed _charactermovement 3e+02)))

(event Input|MouseEvents|LeftMouseButton
  (params (Key :type Key%20Structure :default "None"))
  ;[1 1 1] Attack Animation
  (:Pressed
    (Animation|PlayAnimMontage "/Game/Animations/AttackMove.AttackMove" 1.0 "None")))

(fn ConstructionScript)